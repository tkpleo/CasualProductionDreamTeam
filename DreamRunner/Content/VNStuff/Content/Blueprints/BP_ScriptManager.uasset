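; Visual novel script manager that shows a loading screen, creates the HUD and drives the story forward on left clicks.
; Each step reads a DTScript row for music, background and event type: dialog, focused event, fade-in or background change.
; Message playback pulls speaker, expression, SFX and line from DTDialog using a separate counter, then feeds the HUD widgets.
; MsgEnd shows the proceed prompt, gated on typing and animation flags for focused events.
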(event Custom|Action
  (bind _hud_ref (Variables|Refs|GetHUD%20Ref))
  (bind _wg_dialog (Variables|/Game/VNStuff/Content/UI/WG_HUD.WG_HUD_C|GetWG_Dialog _hud_ref))
  ;[0.15 0.15 0.15 0.5] Action
  (Variables|States|SetCanProceed false)
  (Default|ClearText _wg_dialog)
  (Default|ShowProceed _wg_dialog "Hidden")
  (CallFunction|NextScriptRow)
  (CallFunction|GetScriptRow (Utilities|String|StringToName (Utilities|String|ToString(Integer) (Variables|Counter|GetScript%20Counter))))
  (Utilities|FlowControl|Sequence
    (:then_0
      (switch Utilities|FlowControl|Switch|SwitchonE_Script (Variables|States|GetSpecial%20Event)
        (:NewEnumerator1
          (CallFunction|FocusedEvent))
        (:NewEnumerator2
          (CallFunction|PlayMsg))
        (:NewEnumerator5
          (CallFunction|FadeinEvent))
        (:NewEnumerator6
          (CallFunction|ChangeBackground))))
    (:then_1
      ;;[0.15 0.15 0.15 0.5] If Music is valid then change music
      (if (not (== (Variables|Counter|GetScript%20Counter) 1))
        (CallFunction|PlayMusic)))))

(event Custom|Play%20Msg
  ;[0.15 0.15 0.15 0.5] Play Msg
  (CallFunction|NextDialogRow)
  (CallFunction|FillDialog)
  (Variables|States|SetTyping true)
  (Utilities|FlowControl|Sequence
    (:then_0
      ;;[0.15 0.15 0.15 0.5] If There is SFX Play it
      (Utilities|IsValid (Variables|Info|GetSFX)
        (:Is%20Valid
          (Audio|PlaySound2D (Variables|Info|GetSFX) 1.0 1.0 0.0 0 0))))
    (:then_1
      (CallFunction|SetCharacterExpression)
      (Default|StartMsg (Variables|/Game/VNStuff/Content/UI/WG_HUD.WG_HUD_C|GetWG_Dialog (Variables|Refs|GetHUD%20Ref)) (Utilities|Text|ToText(String) (Variables|Info|GetLine)) (Variables|Info|GetName)))))

(event Custom|Msg%20End
  ;[0.15 0.15 0.15 0.5] End Msg
  (Variables|States|SetTyping false)
  (switch Utilities|FlowControl|Switch|SwitchonE_Script (Variables|States|GetSpecial%20Event)
    (:NewEnumerator1
      (CallFunction|FocusedEventProceedTest))
    (:NewEnumerator2
      (Default|ShowProceed (Variables|/Game/VNStuff/Content/UI/WG_HUD.WG_HUD_C|GetWG_Dialog (Variables|Refs|GetHUD%20Ref)) "Visible" :!label _label)
      (CallFunction|EnableInputAfterFirstRun))
    (:NewEnumerator5
      (goto _label))
    (:NewEnumerator6
      (goto _label))))

(event Custom|Fade%20In%20Event
  (bind _background (Variables|Info|GetBackground))
  (bind _hud_ref (Variables|Refs|GetHUD%20Ref))
  ;[0.15 0.15 0.15 0.5] Fade In Event
  (Utilities|FlowControl|Sequence
    (:then_0
      (Utilities|IsValid _background
        (:Is%20Valid
          (Appearance|SetBrushfromTexture (Variables|/Game/VNStuff/Content/UI/WG_HUD.WG_HUD_C|GetBackground (Variables|Refs|GetHUD%20Ref)) _background false))))
    (:then_1
      (Default|ClearText (Variables|/Game/VNStuff/Content/UI/WG_HUD.WG_HUD_C|GetWG_Dialog _hud_ref))
      (Default|FadeinAnimationPlay (Variables|/Game/VNStuff/Content/UI/WG_HUD.WG_HUD_C|GetWG_Fade _hud_ref)))))

(event Custom|Focused%20Event
  ;[0.15 0.15 0.15 0.5] Focused Event
  (Widget|SetVisibility (Variables|/Game/VNStuff/Content/UI/WG_HUD.WG_HUD_C|GetBackgroundBlur_448 (Variables|Refs|GetHUD%20Ref)) "Visible")
  (CallFunction|PlayMsg)
  (Variables|States|SetFocused%20Active true)
  (Variables|States|SetAnimation%20Playing true)
  (Default|PlayPopAnimation (Variables|/Game/VNStuff/Content/UI/WG_HUD.WG_HUD_C|GetWG_FocusedEvent (Variables|Refs|GetHUD%20Ref)) "Forward" (Utilities|Array|Get(acopy) (Variables|Info|GetFocusedEvent%20Images) (Variables|Counter|GetFocused%20Counter)))
  (Math|Integer|IncrementInt (Variables|Counter|GetFocused%20Counter)))

(event Custom|Hide%20Focused%20Event
  (bind _hud_ref (Variables|Refs|GetHUD%20Ref))
  ;[0.15 0.15 0.15 0.5] Hide Focused Event
  (if (Variables|States|GetFocused%20Active)
    (Default|PlayPopAnimation (Variables|/Game/VNStuff/Content/UI/WG_HUD.WG_HUD_C|GetWG_FocusedEvent _hud_ref) "Reverse")
    (Widget|SetVisibility (Variables|/Game/VNStuff/Content/UI/WG_HUD.WG_HUD_C|GetBackgroundBlur_448 _hud_ref) "Hidden")
    (Variables|States|SetFocused%20Active false)))

(event Custom|Change%20Background
  (bind _hud_ref (Variables|Refs|GetHUD%20Ref))
  ;[0.15 0.15 0.15 0.5] Change Background
  (CallFunction|HideFocusedEvent)
  (Default|HideDialog (Variables|/Game/VNStuff/Content/UI/WG_HUD.WG_HUD_C|GetWG_Dialog _hud_ref))
  (Widget|SetVisibility (Variables|/Game/VNStuff/Content/UI/WG_Character1.WG_Character1_C|GetCharacterImage (Variables|/Game/VNStuff/Content/UI/WG_HUD.WG_HUD_C|GetWG_Character1 _hud_ref)) "Hidden")
  (Default|PlayFadeOutin (Variables|/Game/VNStuff/Content/UI/WG_HUD.WG_HUD_C|GetWG_Fade _hud_ref))
  (Utilities|FlowControl|Delay 0.51)
  (Appearance|SetBrushfromTexture (Variables|/Game/VNStuff/Content/UI/WG_HUD.WG_HUD_C|GetBackground (Variables|Refs|GetHUD%20Ref)) (Variables|Info|GetBackground) false))

(event Custom|Yes%20No
  (Variables|States|SetQuestion%20Msg true)
  (Variables|States|SetYN%20Loop true)
  (Variables|Counter|SetYN%20Counter (+ (Variables|Counter|GetYN%20Counter) 1)))

(event EventBeginPlay
  (bind _returnvalue (UserInterface|CreateWidget "/Game/VNStuff/Content/UI/WG_Loading.WG_Loading_C" (Game|GetPlayerController 0)))
  (bind _output_get (Variables|Refs|SetLoading%20Screen _returnvalue))
  (UserInterface|Viewport|AddtoViewport _output_get 0)
  (Utilities|FlowControl|Delay 2.0)
  (bind _returnvalue_2 (UserInterface|CreateWidget "/Game/VNStuff/Content/UI/WG_HUD.WG_HUD_C" (Game|GetPlayerController 0) self))
  (Variables|Refs|SetHUD%20Ref _returnvalue_2)
  (Widget|RemovefromParent (Variables|Refs|GetLoading%20Screen))
  (UserInterface|Viewport|AddtoViewport (Variables|Refs|GetHUD%20Ref) 0)
  (CallFunction|GetScriptRow "1")
  (Utilities|FlowControl|Sequence
    (:then_0
      (CallFunction|PlayMusic))
    (:then_1
      (Utilities|FlowControl|Delay 1.0)
      (Default|ShowDialog (Variables|/Game/VNStuff/Content/UI/WG_HUD.WG_HUD_C|GetWG_Dialog (Variables|Refs|GetHUD%20Ref))))))

(event Input|MouseEvents|LeftMouseButton
  (params (Key :type Key%20Structure :default "None"))
  ;[0.15 0.15 0.15 0.5] Inputs
  (:Pressed
    (if (Variables|States|GetCanProceed)
      (CallFunction|Action))))

(fn ConstructionScript)

(fn GetScriptRow
  (params (RowName :type Name))
  (bind _returnvalue (Utilities|GetDataTableRow (Variables|DataTables|GetDT_Script) RowName)
    (:then
      (Variables|States|SetSpecial%20Event (.SpecialEvent (Utilities|Struct|BreakST_Script _returnvalue)))
      (Variables|Info|SetMusic (.Music (Utilities|Struct|BreakST_Script _returnvalue)))
      (Variables|Info|SetBackground (.Background (Utilities|Struct|BreakST_Script _returnvalue))))))

(fn PlayMusic
  (bind _background_music (Variables|Default|GetBackground%20Music))
  (Utilities|IsValid (Variables|Info|GetMusic)
    (:Is%20Valid
      (Audio|Components|Audio|SetSound _background_music (Variables|Info|GetMusic))
      (Audio|Components|Audio|FadeIn _background_music 1.0 1.0 0.0 "Linear" :!class /Script/Engine.AudioComponent))))

(fn NextScriptRow
  (Variables|Counter|SetScript%20Counter (+ (Variables|Counter|GetScript%20Counter) 1)))

(fn NextDialogRow
  (Variables|Counter|SetDialog%20Counter (+ (Variables|Counter|GetDialog%20Counter) 1)))

(fn FillDialog
  (bind _returnvalue (Utilities|GetDataTableRow (Variables|DataTables|GetDT_Dialog) (Utilities|String|StringToName (Utilities|String|ToString(Integer) (Variables|Counter|GetDialog%20Counter))))
    (:then
      (Variables|Info|SetName (.Name (Utilities|Struct|BreakST_DialogSetup _returnvalue)))
      (Variables|Info|SetExpression (.Expression (Utilities|Struct|BreakST_DialogSetup _returnvalue)))
      (Variables|Info|SetSFX (.SFX (Utilities|Struct|BreakST_DialogSetup _returnvalue)))
      (Variables|Info|SetLine (.Line (Utilities|Struct|BreakST_DialogSetup _returnvalue))))))

(fn EnableInputAfterFirstRun
  (bind _returnvalue (Game|GetPlayerController 0))
  (if (== (Variables|Counter|GetScript%20Counter) 1)
    (Input|EnableInput _returnvalue)
    (Variables|/Script/Engine.PlayerController|SetbShowMouseCursor _returnvalue true)))

(fn SetCharacterExpression
  (bind _hud_ref (Variables|Refs|GetHUD%20Ref))
  (bind _wg_character1 (Variables|/Game/VNStuff/Content/UI/WG_HUD.WG_HUD_C|GetWG_Character1 _hud_ref))
  (bind _characterimage (Variables|/Game/VNStuff/Content/UI/WG_Character1.WG_Character1_C|GetCharacterImage _wg_character1))
  (Appearance|SetBrushfromTexture _characterimage (Variables|Info|GetExpression) true)
  (Widget|SetVisibility _characterimage "Visible"))

(fn FocusedEventProceedTest
  (if (not (and (Variables|States|GetTyping) (Variables|States|GetAnimation%20Playing)))
    (Default|ShowProceed (Variables|/Game/VNStuff/Content/UI/WG_HUD.WG_HUD_C|GetWG_Dialog (Variables|Refs|GetHUD%20Ref)) "Visible")))